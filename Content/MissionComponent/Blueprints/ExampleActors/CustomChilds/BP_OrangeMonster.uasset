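; BP_OrangeMonster is an example NPC actor in the MissionComponent folder that moves between locations through its BPAIComponent.
; The construction script runs the parent's, then copies the actor's MoveToRandomLocations flag to the component.
; On BeginPlay, after the parent logic, it tells the component to move the NPC to LocationInfo when random movement is off.
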(event `self.ReceiveBeginPlay`
  (`parent.ReceiveBeginPlay`)
  (if (not (`self.Move to Random Locations?`))
    (`/Game/MissionComponent/Blueprints/Components/BP_AIComponent.Move_NPC_To_Locations` (`self.BP_AIComponent`) (`self.Location Info`))))

(fn `UserConstructionScript`
  (`parent.UserConstructionScript`)
  (set `/Game/MissionComponent/Blueprints/Components/BP_AIComponent.MoveToRandomLocations?` (`self.Move to Random Locations?`) (`self.BP_AIComponent`)))